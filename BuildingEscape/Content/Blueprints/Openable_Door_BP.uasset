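; Openable door actor that swings open and closed in response to open and close requests from its OpenDoor events.
; The DoorSwing timeline plays forward to open and reverses to close, adding its OpenAngle yaw to the rotation saved at BeginPlay.
; A Sound Timing event track on the same timeline plays the door lock sound at the actor's location, keeping audio tied to the swing.
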(event `self.ReceiveBeginPlay`
  (`parent.ReceiveBeginPlay`)
  (set `self.InitialRotation` (`self.K2_GetActorRotation`)))

(event `self.OpenDoor.OnOpenRequest`
  (bind (_direction _openangle) (`Timeline|DoorSwing` :!label _label)
    (:`Update`
      (`self.K2_SetActorRotation` (`KismetMathLibrary.ComposeRotators` (`KismetMathLibrary.MakeRotator` 0.0 0.0 _openangle) (`self.InitialRotation`))))
    (:`SoundTiming`
      (`GameplayStatics.PlaySoundAtLocation` "/Game/Audio/door-lock.door-lock" (`self.K2_GetActorLocation`)))))

(event `self.OpenDoor.OnCloseRequest`
  (goto _label :!via `Reverse`))

(fn `UserConstructionScript`
  (`parent.UserConstructionScript`))